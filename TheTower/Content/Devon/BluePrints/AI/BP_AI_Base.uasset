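; BP_AI_Base is a base enemy Blueprint that handles taking damage from the player, dealing hitbox damage and granting XP on death.
; Player damage reduces Health only while that player's EnemyHit flag is unset, then sets it.
; At zero Health it disables movement, briefly delays, awards BaseXP and destroys itself.
; AttackStart and AttackEnd toggle the Hitbox, whose overlaps damage the player; the Attack function is a stub.
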(event OnComponentBeginOverlap(Hitbox)
  (params (OverlappedComponent :type Primitive%20Component%20Object%20Reference) (OtherActor :type Actor%20Object%20Reference) (OtherComp :type Primitive%20Component%20Object%20Reference) (OtherBodyIndex :type Integer) (bFromSweep :type Boolean) (SweepResult :type Hit%20Result%20Structure%20%28by%20ref%29))
  (bind _asbp_player (Utilities|Casting|CastToBP_Player OtherActor))
  (if true
    (Game|Damage|ApplyDamage _asbp_player (Variables|Default|GetAttackDamage) 0 0)
    (Development|PrintString (Utilities|String|ToString(Float) (Variables|/Game/BluePrints/Player/BP_Player.BP_Player_C|GetHealth _asbp_player)))))

(event Custom|Attack%20Start
  (Collision|SetCollisionEnabled (Variables|Default|GetHitbox) "QueryOnly"))

(event Custom|AttackEnd
  (Collision|SetCollisionEnabled (Variables|Default|GetHitbox) "NoCollision"))

(event Game|Damage|EventAnyDamage
  (params (Damage :type Float%20%28single-precision%29) (DamageType :type Damage%20Type%20Object%20Reference) (InstigatedBy :type Controller%20Object%20Reference) (DamageCauser :type Actor%20Object%20Reference))
  (bind _asbp_player (Utilities|Casting|CastToBP_Player DamageCauser))
  (if (not (Variables|/Game/BluePrints/Player/BP_Player.BP_Player_C|GetEnemyHit _asbp_player))
    (Development|PrintString (Utilities|String|ToString(Float) Damage))
    (Variables|Default|SetHealth (- (Variables|Default|GetHealth) Damage))
    (if (<= (Variables|Default|GetHealth) 0.0)
      (Variables|/Game/BluePrints/Player/BP_Player.BP_Player_C|SetEnemyHit _asbp_player true)
      (Pawn|Components|CharacterMovement|DisableMovement (Variables|Character|GetCharacterMovement))
      (Utilities|FlowControl|Delay 0.2)
      (Default|XPCalc _asbp_player (Variables|Default|GetBaseXP))
      (Actor|DestroyActor)
      (else
        (Variables|/Game/BluePrints/Player/BP_Player.BP_Player_C|SetEnemyHit _asbp_player true)))))

(fn ConstructionScript)

(fn Attack
  (return 0.0))