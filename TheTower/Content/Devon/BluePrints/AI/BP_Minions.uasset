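; BP_Minions is a skeleton minion AI character that spawns with a random Blade, Axe or Staff, with Blade weighted double.
; BeginPlay sets full health and calls EquipWeapon, which swaps the weapon mesh and snaps it to the right-hand socket.
; Attack plays and returns the montage matching the weapon type.
; The Heal event restores a fraction of max health, clamps it, and prints the result.
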(event EventBeginPlay
  (bind _output_get (Variables|Default|SetWeaponType (Utilities|Select :Index (Math|Random|RandomIntegerinRange 0 3) :Option%200 "NewEnumerator0" :Option%201 "NewEnumerator1" :Option%202 "NewEnumerator0" :Option%203 "NewEnumerator3")))
  (CallFunction|EquipWeapon _output_get)
  (Variables|Default|SetHealth (Variables|Default|GetMaxHealth)))

(event EventHeal
  (params (Heal%20Percentage :type Float%20%28double-precision%29))
  (bind _output_get (Variables|Default|SetHealth (Math|Float|Clamp(Float) (+ (Variables|Default|GetHealth) (* Heal%20Percentage (Variables|Default|GetMaxHealth))) 0.0 (Variables|Default|GetMaxHealth))))
  (Development|PrintString (Utilities|String|ToString(Float) _output_get)))

(fn ConstructionScript
  (|CallParentFunction))

(fn EquipWeapon
  (params (Weapon%20Type :type E_Weapon%20Enum :default "NewEnumerator0"))
  (bind _weapon (Variables|Default|GetWeapon))
  (Components|StaticMesh|SetStaticMesh _weapon (Utilities|Select :Index Weapon%20Type :NewEnumerator0 "/Game/Devon/Assets/Weapons/Skeleton_Blade.Skeleton_Blade" :NewEnumerator1 "/Game/Devon/Assets/Weapons/Skeleton_Axe.Skeleton_Axe" :NewEnumerator3 "/Game/Devon/Assets/Weapons/Skeleton_Staff.Skeleton_Staff"))
  (Transformation|AttachComponentToComponent _weapon (Variables|Character|GetMesh) "handslot_r" "SnapToTarget" "SnapToTarget" "KeepRelative" true)
  (Transformation|SetRelativeRotation (Variables|Default|GetWeapon) "0.000000,0.000000,-90.000000" false false))

(fn Attack
  (bind _returnvalue (Animation|PlayAnimMontage (Utilities|Select :Index (Variables|Default|GetWeaponType) :NewEnumerator0 "/Game/Devon/BluePrints/Animation/AM_Blade.AM_Blade" :NewEnumerator1 "/Game/Devon/BluePrints/Animation/AM_Axe.AM_Axe" :NewEnumerator3 "/Game/Devon/BluePrints/Animation/AM_Staff.AM_Staff") 1.0 "None"))
  (return _returnvalue))