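; BP_Rogues is a crossbow-wielding AI character that shoots arrows.
; On BeginPlay it snaps the Crossbow component to the mesh's right-hand socket and corrects its rotation.
; Attack plays the crossbow montage, while a separate Fire event spawns BP_Arrow at the Arrow1 component's world transform.
; A Heal event restores a fraction of MaxHealth, clamped to the valid range, and prints the resulting health.
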(event Custom|Fire
  (bind _arrow1 (Variables|Default|GetArrow1))
  (Game|SpawnActorfromClass "/Game/Devon/BluePrints/BP_Arrow.BP_Arrow_C" (Math|Transform|MakeTransform (Transformation|GetWorldLocation _arrow1) (Transformation|GetWorldRotation _arrow1) "1.000000,1.000000,1.000000") "Undefined" "MultiplyWithRoot" 0 0))

(event EventBeginPlay
  (CallFunction|EquipWeapon))

(event EventHeal
  (params (Heal%20Percentage :type Float%20%28double-precision%29))
  (bind _output_get (Variables|Default|SetHealth (Math|Float|Clamp(Float) (+ (Variables|Default|GetHealth) (* Heal%20Percentage (Variables|Default|GetMaxHealth))) 0.0 (Variables|Default|GetMaxHealth))))
  (Development|PrintString (Utilities|String|ToString(Float) _output_get)))

(fn ConstructionScript
  (|CallParentFunction))

(fn EquipWeapon
  (bind _crossbow (Variables|Default|GetCrossbow))
  (Transformation|AttachComponentToComponent _crossbow (Variables|Character|GetMesh) "hand_r" "SnapToTarget" "SnapToTarget" "KeepRelative" true)
  (Transformation|SetRelativeTransform _crossbow (Math|Transform|MakeTransform "0, 0, 0" "-90.000000,-180.000000,0.000000" "1.000000,1.000000,1.000000") false false))

(fn Attack
  (bind _returnvalue (Animation|PlayAnimMontage "/Game/Devon/BluePrints/Animation/AM_Crossbow.AM_Crossbow" 1.0 "None"))
  (return _returnvalue))