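; BP_Collectable is a spinning pickup that grants the player a random boost.
; On BeginPlay, a fast looping timer calls Rotate, which yaws the root component in small steps without using Tick.
; When a BP_ThirdPersonCharacter overlaps its Box, a random bool selects that character's JumpBoost or SpeedBoost, then the collectable destroys itself.
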(event OnComponentBeginOverlap(Box)
  (params (OverlappedComponent :type Primitive%20Component%20Object%20Reference) (OtherActor :type Actor%20Object%20Reference) (OtherComp :type Primitive%20Component%20Object%20Reference) (OtherBodyIndex :type Integer) (bFromSweep :type Boolean) (SweepResult :type Hit%20Result%20Structure%20%28by%20ref%29))
  (bind _asbp_third_person_character (Utilities|Casting|CastToBP_ThirdPersonCharacter OtherActor))
  (if (Math|Random|RandomBool)
    (Default|JumpBoost _asbp_third_person_character)
    (Actor|DestroyActor)
    (else
      (Default|SpeedBoost _asbp_third_person_character)
      (Actor|DestroyActor))))

(event EventBeginPlay
  (Utilities|Time|SetTimerbyFunctionName 0 "Rotate" 0.005 true))

(fn ConstructionScript)

(fn Rotate
  (Transformation|AddLocalRotation (Variables|Default|GetDefaultSceneRoot) (Math|Rotator|MakeRotator 0.0 0.0 0.5) false false))