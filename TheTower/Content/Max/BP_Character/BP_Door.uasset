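; A door that swings open for a character once the game mode reports no collectables left.
; On overlap it reads CollectablesLeft from BP_ThirdPersonGameMode, then either plays a timeline that yaws the door mesh up to a quarter turn or prints a message about needing a key.
; When a character leaves the overlap, the same timeline reverses to swing the door back.
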(event EventBeginPlay)

(event Collision|EventActorBeginOverlap
  (params (OtherActor :type Actor%20Object%20Reference))
  (bind _asbp_third_person_game_mode (Utilities|Casting|CastToBP_ThirdPersonGameMode (Game|GetGameMode)))
  (if (== (Variables|/Game/ThirdPerson/Blueprints/BP_ThirdPersonGameMode.BP_ThirdPersonGameMode_C|GetCollectablesLeft _asbp_third_person_game_mode) 0)
    (Utilities|Casting|CastToCharacter OtherActor)
    (bind _door (Timeline|Door%20Timeline Play)
      (:Update
        (Transformation|SetRelativeRotation (Variables|Default|GetSM_Door) (Math|Rotator|MakeRotator 0.0 0.0 (* _door 9e+01)) false false)))
    (else
      (Development|PrintString "You need to find the key to proceed"))))

(event Collision|EventActorEndOverlap
  (params (OtherActor :type Actor%20Object%20Reference))
  (Utilities|Casting|CastToCharacter OtherActor)
  (bind _door (Timeline|Door%20Timeline Reverse)
    (:Update
      (Transformation|SetRelativeRotation (Variables|Default|GetSM_Door) (Math|Rotator|MakeRotator 0.0 0.0 (* _door 9e+01)) false false))))

(fn ConstructionScript)

(fn GetGamePlayTagContainer
  (return "(TagName=\"\")"))