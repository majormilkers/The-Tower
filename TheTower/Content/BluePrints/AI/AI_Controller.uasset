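; AI controller that runs the BT_AI behavior tree and feeds it player sightings from AI perception.
; Sensing a BP_Player cancels the chase timer and writes Target Player and CanSeePlayer to the blackboard.
; Losing the player starts a looping three-second timer whose EndChase event copies the last stimulus result to CanSeePlayer and sets PlayerLost false, leaving Target Player untouched.
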(event OnTargetPerceptionUpdated(AIPerception)
  (params (Actor :type Actor%20Object%20Reference) (Stimulus :type AI%20Stimulus%20Structure))
  (bind _bsuccessfullysensed (Utilities|Struct|BreakAIStimulus Stimulus))
  (bind _asbp_player (Utilities|Casting|CastToBP_Player Actor))
  (if _bsuccessfullysensed
    (Utilities|Time|ClearandInvalidateTimerbyHandle (Variables|Default|GetClear%20Timer))
    (AI|Components|Blackboard|SetValueasObject (AI|GetBlackboard 0) (Utilities|Name|MakeLiteralName "Target Player") _asbp_player)
    (AI|Components|Blackboard|SetValueasBool (AI|GetBlackboard 0) (Utilities|Name|MakeLiteralName "CanSeePlayer") _bsuccessfullysensed)
    (else
      (bind _returnvalue (Utilities|Time|SetTimerbyEvent (delegate Custom|EndChase) 3.0 true))
      (Variables|Default|SetClear%20Timer _returnvalue))))

(event Custom|EndChase
  (bind _returnvalue (AI|GetBlackboard 0))
  (AI|Components|Blackboard|SetValueasBool _returnvalue (Utilities|Name|MakeLiteralName "CanSeePlayer") (.bSuccessfullySensed (Utilities|Struct|BreakAIStimulus (stale OnTargetPerceptionUpdated(AIPerception) Stimulus))))
  (AI|Components|Blackboard|SetValueasBool _returnvalue (Utilities|Name|MakeLiteralName "PlayerLost") false))

(event EventBeginPlay
  (AI|RunBehaviorTree "/Game/BluePrints/AI/BT_AI.BT_AI"))

(fn ConstructionScript)