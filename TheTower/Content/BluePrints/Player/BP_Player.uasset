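; Player knight pawn with Enhanced Input movement, a HUD, a three-hit melee combo and a montage-driven block.
; TriggerSword starts a looping timer that line-traces between sword sockets, applying damage with a random critical bonus until StopTriggerSword.
; Toggled attack and parry flags keep both actions exclusive, and parrying reduces incoming damage.
; Death plays a montage then quits the game, while XPCalc handles level-ups that restore health.
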(event Custom|TriggerSword
  ;[1 1 1] Melee Attack
  (bind _returnvalue (Utilities|Time|SetTimerbyEvent (delegate Custom|SwordLineTrace) 0.01 true))
  (Variables|Default|SetTriggerSwordEvent _returnvalue))

(event Custom|SwordLineTrace
  ;[1 1 1] Melee Attack
  (bind _outhit (Collision|LineTraceByChannel (Transformation|GetSocketLocation (Variables|Character|GetMesh) "Start") (Transformation|GetSocketLocation (Variables|Character|GetMesh) "End") "TraceTypeQuery2" false 0 "None"))
  (bind _returnvalue (CallFunction|DamageCalc))
  (Game|Damage|ApplyDamage (.HitActor (Collision|BreakHitResult _outhit)) _returnvalue 0 self))

(event Custom|StopTriggerSword
  ;[1 1 1] Melee Attack
  (Variables|Default|SetEnemyHit false)
  (Utilities|Time|ClearandInvalidateTimerbyHandle (Variables|Default|GetTriggerSwordEvent)))

(event Custom|UpdateAttack
  (Variables|Default|SetisAttacking (not (Variables|Default|GetisAttacking))))

(event Custom|UpdateParry
  (Variables|Default|SetisParrying (not (Variables|Default|GetisParrying))))

(event Input|EnhancedActionEvents|EnhancedInputActionIA_MoveLeft
  (params (ActionValue :type Float%20%28double-precision%29) (ElapsedSeconds :type Float%20%28double-precision%29) (TriggeredSeconds :type Float%20%28double-precision%29) (InputAction :type Input%20Action%20Object%20Reference :default "/Game/Input/IA_MoveLeft.IA_MoveLeft"))
  ;[1 1 1] Player Movement Controls
  (Pawn|Input|AddMovementInput (Math|Vector|GetForwardVector (Math|Rotator|MakeRotator 0.0 0.0 (.yaw (Pawn|GetControlRotation :!class /Script/Engine.Pawn)))) ActionValue false))

(event Input|EnhancedActionEvents|EnhancedInputActionIA_MoveForward
  (params (ActionValue :type Float%20%28double-precision%29) (ElapsedSeconds :type Float%20%28double-precision%29) (TriggeredSeconds :type Float%20%28double-precision%29) (InputAction :type Input%20Action%20Object%20Reference :default "/Game/Input/IA_MoveForward.IA_MoveForward"))
  ;[1 1 1] Player Movement Controls
  (Pawn|Input|AddMovementInput (Math|Vector|GetRightVector (Math|Rotator|MakeRotator 0.0 0.0 (.yaw (Pawn|GetControlRotation :!class /Script/Engine.Pawn)))) ActionValue false))

(event EventBeginPlay
  (bind _returnvalue (Game|GetPlayerController 0))
  (bind _returnvalue_2 (PlayerController|LocalPlayerSubsystems|GetEnhancedInputLocalPlayerSubsystem _returnvalue))
  (bind _returnvalue_3 (UserInterface|CreateWidget "/Game/Carlo/UI/WB_HUD.WB_HUD_C" _returnvalue))
  (UserInterface|Viewport|AddtoViewport _returnvalue_3 0)
  (Pawn|Possess _returnvalue self)
  (Utilities|IsValid _returnvalue_2
    (:Is%20Valid
      (Input|AddMappingContext _returnvalue_2 "/Game/Input/IMC_Move.IMC_Move" 0 "(bIgnoreAllPressedKeysUntilRelease=True,bForceImmediately=False,bNotifyUserSettings=False)"))))

(event Game|Damage|EventAnyDamage
  (params (Damage :type Float%20%28single-precision%29) (DamageType :type Damage%20Type%20Object%20Reference) (InstigatedBy :type Controller%20Object%20Reference) (DamageCauser :type Actor%20Object%20Reference))
  (if (Variables|Default|GetisParrying)
    (Audio|PlaySound2D "/Game/Assets/Sound/351372__wilhellboy__lightringingclang.351372__wilhellboy__lightringingclang" 1.0 1.0 0.0 0 0)
    (Variables|Default|SetHealth (- (Variables|Default|GetHealth) (/ (Class|KismetMathLibrary|ToInt64(Float) Damage) 2)))
    (if (<= (Variables|Default|GetHealth) 0.0)
      (Input|DisableInput (Game|GetPlayerController 0))
      (Utilities|FlowControl|DoOnce false
        (:Completed
          (bind _returnvalue (Animation|PlayAnimMontage "/Game/Assets/Characters/Animations/AM_KnightDeath.AM_KnightDeath" 1.0 "None"))
          (Utilities|FlowControl|Delay _returnvalue)
          (Game|QuitGame 0 "Quit" false))))
    (else
      (Variables|Default|SetHealth (- (Variables|Default|GetHealth) Damage))
      (if (<= (Variables|Default|GetHealth) 0.0)
        (Input|DisableInput (Game|GetPlayerController 0))
        (Utilities|FlowControl|DoOnce false
          (:Completed
            (bind _returnvalue_2 (Animation|PlayAnimMontage "/Game/Assets/Characters/Animations/AM_KnightDeath.AM_KnightDeath" 1.0 "None"))
            (Utilities|FlowControl|Delay _returnvalue_2)
            (Game|QuitGame 0 "Quit" false)))))))

(event Input|MouseEvents|LeftMouseButton
  (params (Key :type Key%20Structure :default "None"))
  ;[1 1 1] Melee Attack
  (:Pressed
    (if (not (Variables|Default|GetisParrying))
      (Utilities|FlowControl|DoOnce false :!label _label
        (:Completed
          (if (== (Variables|Default|GetAttackNumber) 0)
            (bind _returnvalue (Animation|PlayAnimMontage "/Game/Assets/Characters/Animations/AM_KnightAttack2.AM_KnightAttack2" 1.0 "None"))
            (Utilities|FlowControl|Delay _returnvalue)
            (Math|Integer|IncrementInt (Variables|Default|GetAttackNumber)
              (:%20%20
                (goto _label Reset)))
            (elif (== (Variables|Default|GetAttackNumber) 1)
              (bind _returnvalue_2 (Animation|PlayAnimMontage "/Game/Assets/Characters/Animations/AM_KnightAttack.AM_KnightAttack" 1.0 "None"))
              (Utilities|FlowControl|Delay _returnvalue_2)
              (Math|Integer|IncrementInt (Variables|Default|GetAttackNumber)
                (:%20%20
                  (goto _label Reset)))
              (else
                (bind _returnvalue_3 (Animation|PlayAnimMontage "/Game/Assets/Characters/Animations/AM_KnightAttack3.AM_KnightAttack3" 1.0 "None"))
                (Utilities|FlowControl|Delay _returnvalue_3)
                (Variables|Default|SetAttackNumber 0)
                (goto _label Reset)))))))))

(event Input|MouseEvents|RightMouseButton
  (params (Key :type Key%20Structure :default "None"))
  (:Pressed
    (if (not (Variables|Default|GetisAttacking))
      (Utilities|FlowControl|DoOnce false :!label _label
        (:Completed
          (bind _returnvalue (Animation|PlayAnimMontage "/Game/Assets/Characters/Animations/AM_KnightBlock.AM_KnightBlock" 1.0 "None"))
          (Utilities|FlowControl|Delay _returnvalue)
          (goto _label Reset))))))

(fn ConstructionScript)

(fn DamageCalc
  (bind _basedamage (Variables|Default|GetBaseDamage))
  (if (<= (Math|Random|RandomFloatinRange 0.0 1e+02) (Variables|Default|GetCriticalChance))
    (return (+ _basedamage (* (/ _basedamage 1e+02) (Variables|Default|GetCriticalDamageMod))))
    (else
      (return (Variables|Default|GetBaseDamage)))))

(fn XPCalc
  (params (XPAmount :type Float%20%28double-precision%29))
  (Variables|Default|SetXP (+ XPAmount (Variables|Default|GetXP)))
  (if (>= (Variables|Default|GetXP) 1e+02)
    (Variables|Default|SetXP (- (Variables|Default|GetXP) 1e+02))
    (Math|Integer|IncrementInt (Variables|Default|GetLevel)
      (:%20%20
        (Variables|Default|SetHealth 1e+02)))))